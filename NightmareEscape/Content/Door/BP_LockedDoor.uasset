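; BP_LockedDoor is a door the player can open and close with Interact while nearby and holding a key.
; The Box overlap caches the ThirdPersonCharacter, toggles input, and opens or closes a Gate around the interaction.
; With HasKey set, a FlipFlop alternately plays and reverses a Timeline that lerps the mesh's yaw between Closed and Open.
; Without the key, it plays a locked-door sound at the actor's location.
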(event `InputAction|Interact`
  (params (Key :type "Key Structure"))
  ;[1 1 1] if Close and Has Key can open Door
  (:`Pressed`
    (if (`/Game/ThirdPersonBP/Blueprints/ThirdPersonCharacter.HasKey` (stale `self.Box.OnComponentBeginOverlap` _asthird_person_character))
      (`/Engine/EditorBlueprintResources/StandardMacros.Gate` true :!label _label
        (:`Exit`
          ;[1 1 1] Open/Close DoorAnimation
          (`/Engine/EditorBlueprintResources/StandardMacros.FlipFlop`
            (:`A`
              (bind (_direction _track_door) (`Timeline|Open/Close Door` :!label _label_2)
                (:`Update`
                  (`SceneComponent.K2_SetRelativeRotation` (`self.StaticMesh`) (`KismetMathLibrary.MakeRotator` 0.0 0.0 (`KismetMathLibrary.Lerp` (`self.Closed`) (`self.Open`) _track_door)) false false))))
            (:`B`
              (goto _label_2 :!via `Reverse`)))))
      (else
        (`GameplayStatics.PlaySoundAtLocation` "/Game/Sounds/LockedDoor.LockedDoor" (`self.K2_GetActorLocation`) (struct) 1.0 1.0 0.0 null null null)))))

(event `self.Box.OnComponentBeginOverlap`
  (params (OverlappedComponent :type "PrimitiveComponent Object Reference") (OtherActor :type "Actor Object Reference") (OtherComp :type "PrimitiveComponent Object Reference") (OtherBodyIndex :type Integer) (bFromSweep :type Boolean) (SweepResult :type "HitResult Structure (by ref)"))
  ;[1 1 1] if Close and Has Key can open Door
  (bind _asthird_person_character (cast `/Game/ThirdPersonBP/Blueprints/ThirdPersonCharacter` OtherActor))
  (`self.EnableInput` (`GameplayStatics.GetPlayerController` 0))
  (goto _label :!via `Open`))

(event `self.Box.OnComponentEndOverlap`
  (params (OverlappedComponent :type "PrimitiveComponent Object Reference") (OtherActor :type "Actor Object Reference") (OtherComp :type "PrimitiveComponent Object Reference") (OtherBodyIndex :type Integer))
  ;[1 1 1] if Close and Has Key can open Door
  (cast `/Game/ThirdPersonBP/Blueprints/ThirdPersonCharacter` OtherActor)
  (`self.DisableInput` (`GameplayStatics.GetPlayerController` 0))
  (goto _label :!via `Close`))

(fn `UserConstructionScript`)