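; BP_Key is a colour-coded key pickup for the third-person character.
; Box overlap immediately inserts true into the character's HasKey at KeyValue and shows a timed Key_pickup widget, guarded by a DoOnce.
; Overlap also enables input and opens a Gate, so Interact sets KeyCollect, plays a sound and destroys the key; leaving reverses this.
; The construction script applies the chosen mesh and a coloured dynamic material.
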(event `self.Box.OnComponentBeginOverlap`
  (params (OverlappedComponent :type "PrimitiveComponent Object Reference") (OtherActor :type "Actor Object Reference") (OtherComp :type "PrimitiveComponent Object Reference") (OtherBodyIndex :type Integer) (bFromSweep :type Boolean) (SweepResult :type "HitResult Structure (by ref)"))
  (bind _asthird_person_character (cast `/Game/ThirdPersonBP/Blueprints/ThirdPersonCharacter` OtherActor))
  (`|ExecutionSequence`
    (:`then_0`
      (`KismetArrayLibrary.Array_Insert` (`/Game/ThirdPersonBP/Blueprints/ThirdPersonCharacter.HasKey` _asthird_person_character) true (`self.Key Value`))
      (`/Engine/EditorBlueprintResources/StandardMacros.DoOnce` false :!label _label
        (:`Completed`
          (bind _returnvalue (`|CreateWidget` "/Game/DoorAndKeys/Key_pickup.Key_pickup_C"))
          (set `/Game/DoorAndKeys/Key_pickup.Colour` (`self.Key Colour`) _returnvalue)
          (`UserWidget.AddToViewport` _returnvalue 0)
          (`KismetSystemLibrary.Delay` 3.0)
          (`Widget.RemoveFromParent` _returnvalue)
          (goto _label :!via `Reset`))))
    (:`then_1`
      (`self.EnableInput` (`GameplayStatics.GetPlayerController` 0))
      (goto _label_2 :!via `Open`))))

(event `InputAction|Interact`
  (params (Key :type "Key Structure"))
  (:`Pressed`
    (`/Engine/EditorBlueprintResources/StandardMacros.Gate` false :!label _label_2
      (:`Exit`
        (set `/Game/ThirdPersonBP/Blueprints/ThirdPersonCharacter.KeyCollect` true (stale `self.Box.OnComponentBeginOverlap` _asthird_person_character))
        (`GameplayStatics.PlaySoundAtLocation` "/Game/Sounds/KeyPickupSound.KeyPickupSound" (`self.K2_GetActorLocation`) (struct) 1.0 1.0 0.0 null null null)
        (`self.K2_DestroyActor`)))))

(event `self.Box.OnComponentEndOverlap`
  (params (OverlappedComponent :type "PrimitiveComponent Object Reference") (OtherActor :type "Actor Object Reference") (OtherComp :type "PrimitiveComponent Object Reference") (OtherBodyIndex :type Integer))
  (cast `/Game/ThirdPersonBP/Blueprints/ThirdPersonCharacter` OtherActor)
  (`self.DisableInput` (`GameplayStatics.GetPlayerController` 0))
  (goto _label_2 :!via `Close`))

(fn `UserConstructionScript`
  (bind _staticmesh (`self.StaticMesh`))
  (`StaticMeshComponent.SetStaticMesh` _staticmesh (`self.KeyMesh`))
  (bind _returnvalue (`PrimitiveComponent.CreateDynamicMaterialInstance` _staticmesh 0 (`self.KeyMaterial`) "None"))
  (`MaterialInstanceDynamic.SetVectorParameterValue` _returnvalue "Colour" (`self.Colour`))
  (`PrimitiveComponent.SetMaterial` _staticmesh 0 _returnvalue))