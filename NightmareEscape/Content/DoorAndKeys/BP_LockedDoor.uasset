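; Locked door actor that a ThirdPersonCharacter opens and closes with Interact, with mesh and tinted dynamic material set at construction.
; A box overlap enables input and opens a gate.
; If KeyCollect is true, a FlipFlop drives a timeline yaw swing, resetting the KeyValue slot in HasKey after opening.
; Otherwise it plays a locked sound and briefly shows a wrong-or-no-key widget.
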(event `InputAction|Interact`
  (params (Key :type "Key Structure"))
  ;[1 1 1] If you dont have the key/right key text prompt
  (:`Pressed`
    (if (`/Game/ThirdPersonBP/Blueprints/ThirdPersonCharacter.KeyCollect` (stale `self.Box.OnComponentBeginOverlap` _asthird_person_character))
      (`/Engine/EditorBlueprintResources/StandardMacros.Gate` true :!label _label
        (:`Exit`
          (`/Engine/EditorBlueprintResources/StandardMacros.FlipFlop`
            (:`A`
              (bind (_direction _track_door) (`Timeline|Open/Close Door` :!label _label_2)
                (:`Update`
                  (`SceneComponent.K2_SetRelativeRotation` (`self.StaticMesh`) (`KismetMathLibrary.MakeRotator` 0.0 0.0 (`KismetMathLibrary.Lerp` (`self.Closed`) (`self.Open`) _track_door)) false false))
                (:`Finished`
                  (`KismetSystemLibrary.Delay` 1.0)
                  (`KismetArrayLibrary.Array_Set` (`/Game/ThirdPersonBP/Blueprints/ThirdPersonCharacter.HasKey` (stale `self.Box.OnComponentBeginOverlap` _asthird_person_character)) (`self.Key Value`)))))
            (:`B`
              (goto _label_2 :!via `Reverse`)))))
      (else
        (`GameplayStatics.PlaySoundAtLocation` "/Game/DoorAndKeys/Cue_LockedDoor.Cue_LockedDoor" (`self.K2_GetActorLocation`) (struct) 1.0 1.0 0.0 null null null)
        (`/Engine/EditorBlueprintResources/StandardMacros.DoOnce` false :!label _label_3
          (:`Completed`
            (bind _returnvalue (`|CreateWidget` "/Game/DoorAndKeys/WrongOrNoKey.WrongOrNoKey_C"))
            (`UserWidget.AddToViewport` _returnvalue 0)
            (`KismetSystemLibrary.Delay` 4.0)
            (`Widget.RemoveFromParent` _returnvalue)
            (goto _label_3 :!via `Reset`)))))))

(event `self.Box.OnComponentBeginOverlap`
  (params (OverlappedComponent :type "PrimitiveComponent Object Reference") (OtherActor :type "Actor Object Reference") (OtherComp :type "PrimitiveComponent Object Reference") (OtherBodyIndex :type Integer) (bFromSweep :type Boolean) (SweepResult :type "HitResult Structure (by ref)"))
  ;[1 1 1] If you dont have the key/right key text prompt
  (bind _asthird_person_character (cast `/Game/ThirdPersonBP/Blueprints/ThirdPersonCharacter` OtherActor))
  (`/Engine/EditorBlueprintResources/StandardMacros.DoOnce` false :!label _label_4
    (:`Completed`
      (`|ExecutionSequence`
        (:`then_0`
          (`self.EnableInput` (`GameplayStatics.GetPlayerController` 0))
          (goto _label :!via `Open`))
        (:`then_1`
          (for (_array_element _array_index) (`/Game/ThirdPersonBP/Blueprints/ThirdPersonCharacter.HasKey` _asthird_person_character)
            _)
          (if (not (and _array_element (== _array_index (`self.Key Value`))))
            (`|ExecutionSequence`
              (:`then_1`
                (goto _label_4 :!via `Reset`)))))))))

(event `self.Box.OnComponentEndOverlap`
  (params (OverlappedComponent :type "PrimitiveComponent Object Reference") (OtherActor :type "Actor Object Reference") (OtherComp :type "PrimitiveComponent Object Reference") (OtherBodyIndex :type Integer))
  ;[1 1 1] If you dont have the key/right key text prompt
  (cast `/Game/ThirdPersonBP/Blueprints/ThirdPersonCharacter` OtherActor)
  (`self.DisableInput` (`GameplayStatics.GetPlayerController` 0))
  (goto _label :!via `Close`))

(fn `UserConstructionScript`
  (bind _staticmesh (`self.StaticMesh`))
  (`StaticMeshComponent.SetStaticMesh` _staticmesh (`self.DoorMesh`))
  (bind _returnvalue (`PrimitiveComponent.CreateDynamicMaterialInstance` _staticmesh 0 (`self.Material`) "None"))
  (`MaterialInstanceDynamic.SetVectorParameterValue` _returnvalue "Colour" (`self.Colour`))
  (`PrimitiveComponent.SetMaterial` _staticmesh 0 _returnvalue))